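; VR hand actor for BP_Gorilla's Gorilla Tag-style, arm-driven locomotion, following its motion controller.
; Pass, Final and Unstick form the movement steps, sphere-casting from the last hand position toward an arm-length-clamped target to yield push offsets, track contact and release stuck hands.
; The Follower component snaps to that resolved position through OnRep_Last.
; Tick also measures body-relative hand velocity for future throwing and fires one haptic pulse per contact.
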(event `self.ReceiveBeginPlay`
  (`/Engine/EditorBlueprintResources/StandardMacros.IsValid` (`Actor.Instigator` (`self.GetOwner`)) :!label _label
    (:`Is Valid`
      (bind _asbp_gorilla (cast `/Game/GorillaLocomotion_UE4Port/Blueprints/BP_Gorilla` (`Actor.Instigator` (`self.GetOwner`)))
        (:`then`
          (set `self.As BP Gorilla` _asbp_gorilla)
          (set `self.Last` (`self.GetTarget`))
          (set `self.LastHeadPosition` (`self.GetCameraLocation`))
          (set `self.LastPosition` (`self.K2_GetActorLocation` (`self.As BP Gorilla`)))
          (bind _asplayer_controller (cast `PlayerController` (`Pawn.GetController` (`self.As BP Gorilla`)) :!label _label_2)
            (:`then`
              (set `self.As Player Controller` _asplayer_controller))
            (:`CastFailed`
              (`KismetSystemLibrary.Delay` 0.2)
              (goto _label_2))))
        (:`CastFailed`
          (`KismetSystemLibrary.Delay` 0.2 :!label _label_3)
          (goto _label))))
    (:`Is Not Valid`
      (goto _label_3))))

(event `self.ReceiveTick`
  (params (DeltaSeconds :type "Float (single-precision)"))
  (set `self.DeltaSeconds` DeltaSeconds)
  (`KismetSystemLibrary.DrawDebugSphere` (`SceneComponent.K2_GetComponentLocation` (`self.Follower`)) 10.0 12 (struct :`R` 1.0 :`G` 1.0 :`B` 1.0 :`A` 1.0) 0.01 2.0)
  (`self.K2_SetActorLocationAndRotation` (`self.GetControllerLocation`) (struct) false true)
  (`|ExecutionSequence`
    (:`then_0`
      ;[0 0 0] We can use this for caculating throwing speed's
      (bind _as_bp_gorilla (`self.As BP Gorilla`)
        (:`then`
          (if (`Pawn.IsLocallyControlled` _as_bp_gorilla)
            (set `self.VelocityVector` (/ (- (- (`SceneComponent.K2_GetComponentLocation` (`self.Follower`)) (`self.K2_GetActorLocation` (`self.As BP Gorilla`))) (`self.LastHandPosition`)) (`self.DeltaSeconds`)))
            (set `self.Velocity` (`KismetMathLibrary.VSize` (`self.VelocityVector`)))
            (set `self.LastHandPosition` (- (`SceneComponent.K2_GetComponentLocation` (`self.Follower`)) (`self.K2_GetActorLocation` (`self.As BP Gorilla`))))
            (`KismetSystemLibrary.PrintString` (`KismetStringLibrary.Conv_DoubleToString` (`self.Velocity`)) true true (struct :`G` 0.66 :`B` 1.0 :`A` 1.0) 0.0)))
        (:`else`)))
    (:`then_1`
      ;[0 0 0] This Fires A Haptic Effect On The Owning Controller Once The Player Touches The Ground
      (`self.MotionController`
        (:`then`
          (if (`self.GetEngaged`)
            (`/Engine/EditorBlueprintResources/StandardMacros.DoOnce` false :!label _label_4 ; Insures we don't fire multiple haptic effects at once
              (:`Completed`
                (`PlayerController.PlayHapticEffect` (`self.As Player Controller`) "/Game/GorillaLocomotion_UE4Port/Haptics/HandHitHaptic.HandHitHaptic" (`MotionControllerComponent.Hand` (`self.MotionController`)) 0.5 false)))
            (else
              (goto _label_4 :!via `Reset`))))
        (:`else`)))))

(event `Pass - Multicast`
  ;[1 0 0] RPC Events - Depecrated
  (`self.Pass`))

(event `FInal - Mutlicast`
  (params (OtherHandEngaged :type Boolean))
  ;[1 0 0] RPC Events - Depecrated
  (`self.Final` OtherHandEngaged))

(event `Unstick - Multicast`
  ;[1 0 0] RPC Events - Depecrated
  (`self.Unstick`))

(fn `Final`
  (params (OtherHandEngaged :type Boolean))
  (bind (_hit _endposition) (`/Game/GorillaLocomotion_UE4Port/Blueprints/BFL_TraceLib.IterativeCollisionSphereCast` (`self.Last`) (`self.RayCastDistance`) (- (`self.GetTarget`) (`self.Last`)) 0.995 (not (and (`self.GetEngaged`) (`local.OtherHandEngaged`))) (`|MakeArray` (`self.As BP Gorilla`) self :!type "Actor Object Reference")))
  (set `self.Last` (select `bool` _hit :`false` (`self.GetTarget`) :`true` _endposition))
  (set `self.Colliding` (or (`self.Colliding`) _hit)))

(fn `GetCameraLocation`
  (returns (ReturnValue :type "Vector Structure"))
  (return (`SceneComponent.K2_GetComponentLocation` (`/Game/GorillaLocomotion_UE4Port/Blueprints/BP_Gorilla.Camera` (`self.As BP Gorilla`)))))

(fn `GetControllerLocation`
  (returns (ReturnValue :type "Vector Structure"))
  (return (`SceneComponent.K2_GetComponentLocation` (`self.MotionController`))))

(fn `GetControllerRotation`
  (returns (ReturnValue :type "Rotator Structure"))
  (return (`SceneComponent.K2_GetComponentRotation` (`self.MotionController`))))

(fn `GetEngaged`
  (returns (Engaged :type Boolean))
  (return (or (`self.Colliding`) (`self.WasTouching`))))

(fn `GetTarget`
  (returns (Output :type "Vector Structure"))
  (return (+ (`self.GetCameraLocation`) (`KismetMathLibrary.ClampVectorSize` (- (+ (`self.GetControllerLocation`) (`KismetMathLibrary.GreaterGreater_VectorRotator` (`self.Offset`) (`self.GetControllerRotation`))) (`self.GetCameraLocation`)) 0.0 (`/Game/GorillaLocomotion_UE4Port/Blueprints/BP_Gorilla.MaxArmLength` (`self.As BP Gorilla`))))))

(fn `OnRep_As BP Gorilla`)

(fn `OnRep_Last`
  (`SceneComponent.K2_SetWorldLocation` (`self.Follower`) (`self.Last`) false true))

(fn `Pass`
  (returns (First :type "Vector Structure"))
  (bind _deltaseconds (`self.DeltaSeconds`))
  (bind _colliding (`self.Colliding`))
  (bind (_hit _endposition) (`/Game/GorillaLocomotion_UE4Port/Blueprints/BFL_TraceLib.IterativeCollisionSphereCast` (`self.Last`) (`self.RayCastDistance`) (+ (- (`self.GetTarget`) (`self.Last`)) (`KismetMathLibrary.MakeVector` 0.0 0.0 (* -1960.0 _deltaseconds _deltaseconds))) 0.995 true (`|MakeArray` self (`self.As BP Gorilla`) :!type "Actor Object Reference")))
  (set `self.Colliding` _hit)
  (bind _output_get (set `self.First` (select `bool` _colliding :`true` (- (select `bool` (`self.WasTouching`) :`false` _endposition :`true` (`self.Last`)) (`self.GetTarget`)))))
  (`KismetSystemLibrary.PrintString` (`KismetStringLibrary.Concat_StrStr` "MOVEMENT(Hand.First): " (`KismetStringLibrary.Conv_VectorToString` (`self.First`)) " MOVEMENT(Hand.First)Is'Colliding'True?: " (`KismetStringLibrary.Conv_BoolToString` _colliding)) true true (struct :`G` 0.66 :`B` 1.0 :`A` 1.0) 0.0)
  (return _output_get))

(fn `Unstick`
  (bind (_hit _hitresult) (`/Game/GorillaLocomotion_UE4Port/Blueprints/BFL_TraceLib.SafeTrace` (`self.GetCameraLocation`) (+ (`self.GetCameraLocation`) (`/Game/GorillaLocomotion_UE4Port/Blueprints/BFL_TraceLib.ExtendVector` (- (`self.GetTarget`) (`self.GetCameraLocation`)) (`self.RayCastDistance`))) (* (`self.RayCastDistance`) 0.995) (`|MakeArray` (`self.As BP Gorilla`) self :!type "Actor Object Reference")))
  (if (and (and (`self.Colliding`) (> (`KismetMathLibrary.VSize` (- (`self.GetTarget`) (`self.Last`))) (`self.UnstickDistance`))) _hit)
    (set `self.Last` (`self.GetTarget`))
    (set `self.Colliding` false))
  (set `self.WasTouching` (`self.Colliding`))
  (`KismetSystemLibrary.PrintString` (`KismetSystemLibrary.GetDisplayName` (`.HitActor` (`GameplayStatics.BreakHitResult` _hitresult))) true true (struct :`G` 0.66 :`B` 1.0 :`A` 1.0) 0.01))

(fn `UserConstructionScript`)