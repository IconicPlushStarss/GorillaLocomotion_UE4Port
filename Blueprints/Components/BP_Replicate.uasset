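; Deprecated replication component that syncs world transforms of scene components on its owner, defaulting to all of them if none are set.
; Every tick it sends each transform through a server event, which relays it to other clients.
; Receivers passing the control and authority check apply it with teleport, optionally interpolating from the last transform cached in a per-component map.
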(event `self.ReceiveBeginPlay`
  ;[1 0 0 1 100] DEPRECATED
  (if (not (`KismetArrayLibrary.Array_IsValidIndex` (`self.ComponentsToReplicate`)))
    (set `self.ComponentsToReplicate` (`Actor.K2_GetComponentsByClass` (`self.GetOwner`) "/Script/Engine.SceneComponent")))
  (set `self.Tick` true))

(event `self.ReceiveTick`
  (params (DeltaSeconds :type "Float (single-precision)"))
  ;[1 0 0 1 100] DEPRECATED
  (if (`self.Tick`)
    (for _array_element (`self.ComponentsToReplicate`)
      (`self.ReplicateComponentLocation` _array_element (`self.AllowInterpolation?`)))))

(event `ReplicateComponentLocation`
  (params (Component :type "SceneComponent Object Reference") (Interpolate :type Boolean))
  ;[1 0 0 1 100] DEPRECATED
  ;;[1 0 0 1 30] Replicate Components Transforms
  (`self.ReplicateComponentLocation - Server` Component (`SceneComponent.K2_GetComponentToWorld` Component) Interpolate))

(event `ReplicateComponentLocation - Server`
  (params (Component :type "SceneComponent Object Reference") (Transform :type "Transform Structure") (Interp :type Boolean))
  ;[1 0 0 1 100] DEPRECATED
  ;;[1 0 0 1 30] Replicate Components Transforms
  (`self.ReplicateComponentLocation - OtherClients` Component Transform Interp)
  (if (`Actor.HasAuthority` (`self.GetOwner`))
    (`BlueprintMapLibrary.Map_Add` (`self.ReplicatedComponents`) Component Transform)))

(event `ReplicateComponentLocation - OtherClients`
  (params (Component :type "SceneComponent Object Reference") (Transform :type "Transform Structure") (Interp :type Boolean))
  (bind _returnvalue (select `bool` (and Interp (`BlueprintMapLibrary.Map_Contains` (`self.ReplicatedComponents`) Component)) :`false` Transform :`true` (`KismetMathLibrary.TInterpTo` (`BlueprintMapLibrary.Map_Find` (`self.ReplicatedComponents`) Component) Transform (`GameplayStatics.GetWorldDeltaSeconds`) (`self.InterpolationSpeed`))))
  ;[1 0 0 1 100] DEPRECATED
  ;;[1 0 0 1 30] Replicate Components Transforms
  (if (`self.AllowReplication?`)
    (`BlueprintMapLibrary.Map_Add` (`self.ReplicatedComponents`) Component _returnvalue)
    (`SceneComponent.K2_SetWorldTransform` Component _returnvalue false true)))

(fn `AllowReplication?`
  (returns (ReturnValue :type Boolean))
  (return (or (and (not (`Pawn.IsLocallyControlled` (`Actor.Instigator` (`self.GetOwner`)))) (`Pawn.IsLocallyControlled` (`GameplayStatics.GetPlayerPawn` 0))) (and (not (`self.OwnedByPlayer?`)) (not (`Actor.HasAuthority` (`self.GetOwner`)))))))

(fn `OnRep_ComponentsToReplicate`)